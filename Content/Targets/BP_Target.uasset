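; BP_Target is a damageable target with HP that holds pools of Points and Style Points.
; BeginPlay sets the starting values, and Tick destroys the actor once HP reaches zero or below.
; CalculatePointsEarned pays out both pools in proportion to damage against current HP, or everything left on overkill.
; It only returns earned and remaining values, without writing them back to the target.
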(event EventBeginPlay
  (Variables|Default|SetHP 2e+01)
  (Variables|Default|SetPoints 1e+02)
  (Variables|Default|SetStyle%20Points 5e+01))

(event Collision|EventActorBeginOverlap
  (params (OtherActor :type Actor%20Object%20Reference)))

(event EventTick
  (params (DeltaSeconds :type Float%20%28single-precision%29))
  (if (<= (Variables|Default|GetHP) 0.0)
    (Actor|DestroyActor)))

(fn ConstructionScript)

(fn CalculatePointsEarned
  (params (Damage :type Integer))
  (bind _points (Variables|Default|GetPoints))
  (bind _style_points (Variables|Default|GetStyle%20Points))
  (bind _hp (Variables|Default|GetHP))
  (bind _returnvalue (- _hp Damage))
  (bind _returnvalue_2 (/ _returnvalue _hp))
  (bind _returnvalue_3 (* _returnvalue_2 _style_points))
  (bind _returnvalue_4 (* _returnvalue_2 _points))
  (bind _returnvalue_5 (- _style_points _returnvalue_3))
  (bind _returnvalue_6 (- _points _returnvalue_4))
  (bind _returnvalue_7 (Math|Float|Round _returnvalue_6))
  (if (<= _returnvalue_6 _points)
    (return _returnvalue_7 (Math|Float|Truncate _returnvalue_5) (Math|Float|Round _returnvalue) (- (Math|Float|Round _points) _returnvalue_7) (- (Math|Float|Round _style_points) (Math|Float|Round _returnvalue_5))) ; return earned points
    (else
      (return (Math|Float|Round _points) (Math|Float|Truncate (Variables|Default|GetStyle%20Points)) 0 0 0) ; return all points left
    )))